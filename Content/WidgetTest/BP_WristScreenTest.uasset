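; BP_WristScreenTest is a test Blueprint that exercises the BP_WristScreen widget with randomized sprint task data.
; BeginPlay creates the widget and adds it to the viewport.
; Tick accumulates delta time and, every three seconds or so, calls LoadScreen with a random SPrint struct (placeholder task name, progress values, optional extension) and a random task number.
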(event `self.ReceiveBeginPlay`
  (bind _returnvalue (`|CreateWidget` "/Game/Code/wristGadget/WristScreen/BP_WristScreen.BP_WristScreen_C" self))
  (`UserWidget.AddToViewport` _returnvalue 0)
  (set `self.WristScreen` _returnvalue))

(event `self.ReceiveTick`
  (params (DeltaSeconds :type "Float (single-precision)"))
  (bind _output_get (set `self.Counter` (+ DeltaSeconds (`self.Counter`))))
  (if (> _output_get 3.0)
    (set `self.Counter` 0.0)
    (`/Game/Code/wristGadget/WristScreen/BP_WristScreen.LoadScreen` (`self.WristScreen`) (make `/Game/Core/S_Print` (select `int` (`KismetMathLibrary.RandomInteger` 4) :`0` "Grab sbahj collection" :`1` "fire everyone" :`2` "give spongebob his drivers license" :`3` "bet on the rockies" :!type "Name") (`KismetMathLibrary.RandomInteger` 4) 3 (`KismetMathLibrary.RandomInteger` 4) 3 (`KismetMathLibrary.RandomBool`)) (+ (`KismetMathLibrary.RandomInteger` 3) 1))))

(fn `UserConstructionScript`)