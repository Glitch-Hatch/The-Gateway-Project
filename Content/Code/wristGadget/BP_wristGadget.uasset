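; Wrist gadget actor that assigns the player two tasks and offers overlap-driven buttons for screen cycling and level travel.
; On BeginPlay it rolls against TaskArray ranges and call counts to fill TaskSelected, re-rolling recursively if task two repeats task one's name.
; It copies the selection to every BP_text actor, whose three screens one button cycles.
; The other button opens the GatewayPreset level when the player pawn overlaps it.
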(event `self.ReceiveBeginPlay`
  (`self.Set Task1`)
  (`self.Set Task 2`)
  (bind _outactors (`GameplayStatics.GetAllActorsOfClass` "/Game/Code/wristGadget/RenderTargets/BP_text.BP_text_C"))
  (for _array_element _outactors
    (bind _asbp_text (cast `/Game/Code/wristGadget/RenderTargets/BP_text` _array_element))
    (set `/Game/Code/wristGadget/RenderTargets/BP_text.Tasks Used` (`self.Task Selected`) _asbp_text)))

(event `self.WristGear19_Joined-LeftHandFix__Button_003.OnComponentBeginOverlap`
  (params (OverlappedComponent :type "PrimitiveComponent Object Reference") (OtherActor :type "Actor Object Reference") (OtherComp :type "PrimitiveComponent Object Reference") (OtherBodyIndex :type Integer) (bFromSweep :type Boolean) (SweepResult :type "HitResult Structure (by ref)"))
  (`KismetSystemLibrary.PrintString` "Next Wristgear" true true (struct :`R` 1.0 :`B` 0.786115 :`A` 1.0) 5.0)
  (bind _outactors (`GameplayStatics.GetAllActorsOfClass` "/Game/Code/wristGadget/RenderTargets/BP_text.BP_text_C"))
  (for _array_element _outactors
    (bind _displayed_screen (`/Game/Code/wristGadget/RenderTargets/BP_text.displayed screen` _array_element))
    (if (< _displayed_screen 3)
      (set `/Game/Code/wristGadget/RenderTargets/BP_text.displayed screen` (+ _displayed_screen 1) _array_element)
      (else
        (set `/Game/Code/wristGadget/RenderTargets/BP_text.displayed screen` 1 _array_element)))
    (`/Game/Code/wristGadget/RenderTargets/BP_text.Update` _array_element)))

(event `self.WristGear19_Joined-LeftHandFix__Button_001.OnComponentBeginOverlap`
  (params (OverlappedComponent :type "PrimitiveComponent Object Reference") (OtherActor :type "Actor Object Reference") (OtherComp :type "PrimitiveComponent Object Reference") (OtherBodyIndex :type Integer) (bFromSweep :type Boolean) (SweepResult :type "HitResult Structure (by ref)"))
  (if (== OtherActor (`GameplayStatics.GetPlayerPawn` 0))
    (`GameplayStatics.OpenLevelBySoftObjectPtr` "/Game/Core/Levels/GatewayPreset.GatewayPreset")))

(fn `Set Task 2`
  (bind _task2_ (`self.task2%`))
  (bind _task_selected (`self.Task Selected`))
  (set `self.task2%` (`KismetMathLibrary.RandomIntegerInRange` 1 75))
  (for _array_element (`self.TaskArray`)
    (bind (_taskname _minrange _maxrange _timescallable _tasktype _boxneeded1 _boxneeded2 _2parttask_ _timescalled) (break `/Game/Core/S_tasks` _array_element))
    (if (and (<= _minrange _task2_) (>= _maxrange _task2_))
      (if (< _timescallable _timescalled)
        (if (== _taskname (`.TaskName_6_E1D2614A80418031F464488B1C001021` (break `/Game/Core/S_TaskSelected` (`|GetArrayItem` (`self.Task Selected`) 1))))
          (`self.Set Task 2`)
          (else
            (set `self.Task Selected` (`|MakeArray` (`|GetArrayItem` _task_selected) (`|GetArrayItem` _task_selected 1) (make `/Game/Core/S_TaskSelected` 2 _taskname _tasktype _boxneeded1 _boxneeded2 _2parttask_)))))
        (else
          (break)))
      (else
        (break)))))

(fn `Set Task1`
  (bind _task1_ (`self.task1%`))
  (bind _task_selected (`self.Task Selected`))
  (set `self.task1%` (`KismetMathLibrary.RandomIntegerInRange` 1 75))
  (for _array_element (`self.TaskArray`)
    (bind (_taskname _minrange _maxrange _timescallable _tasktype _boxneeded1 _boxneeded2 _2parttask_ _timescalled) (break `/Game/Core/S_tasks` _array_element))
    (if (and (<= _minrange _task1_) (>= _maxrange _task1_))
      (if (< _timescallable _timescalled)
        (set `self.Task Selected` (`|MakeArray` (`|GetArrayItem` _task_selected) (make `/Game/Core/S_TaskSelected` 1 _taskname _tasktype _boxneeded1 _boxneeded2 _2parttask_) (`|GetArrayItem` _task_selected 2)))
        (else
          (break)))
      (else
        (break)))))

(fn `UserConstructionScript`)