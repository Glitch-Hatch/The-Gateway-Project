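; BP_TaskUpdate is an unfinished trigger box, apparently meant to update wrist gadget tasks when a bag enters it.
; On overlap, it gets all BP_Bags actors and loops until one matches the overlapping actor, then does nothing further.
; Reads of the bag type, task text and task integers are left unconnected.
; An author note bars placing it in the loading level.
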(event `self.Box.OnComponentBeginOverlap`
  (params (OverlappedComponent :type "PrimitiveComponent Object Reference") (OtherActor :type "Actor Object Reference") (OtherComp :type "PrimitiveComponent Object Reference") (OtherBodyIndex :type Integer) (bFromSweep :type Boolean) (SweepResult :type "HitResult Structure (by ref)"))
  ; DONOT PLACE IN LOADING LEVEL
  ; get box that went into the hitbox, and what it is full of
  (bind _outactors (`GameplayStatics.GetAllActorsOfClass` "/Game/Code/Bags_And_Locking/Bags/BP_Bags.BP_Bags_C"))
  (for _array_element _outactors
    (if (== _array_element OtherActor)
      (break))))

(fn `UserConstructionScript`)