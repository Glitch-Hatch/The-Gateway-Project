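; BP_Bags is a grabbable bag whose size enum sets its mesh and text labels, and which snaps into matching BP_BagSlot actors.
; Unless a level is loading, BeginPlay places it in a free same-size slot.
; Overlapping a free slot highlights it; dropping there runs chained timelines that rotate, then move the bag in.
; Slotting and removal adjust the PC_Base task counter and refresh BP_text, with separate handling during the trash task.
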(event `self.ReceiveBeginPlay`
  (`KismetSystemLibrary.DelayUntilNextTick`)
  (if (not (`/Game/Core/PC_Base.LoadingLevel?` (cast `/Game/Core/PC_Base` (`GameplayStatics.GetPlayerController` 0) :!pure true)))
    (`PrimitiveComponent.SetEnableGravity` (`self.staticMesh`) false)
    (bind _outactors (`GameplayStatics.GetAllActorsOfClass` "/Game/Code/Bags_And_Locking/Locking/BP_BagSlot.BP_BagSlot_C"))
    (for _array_element _outactors
      (if (`|EnumEquality` (`/Game/Code/Bags_And_Locking/Locking/BP_BagSlot.BagSizeEnum` _array_element) (`self.enum`))
        (if (not (`/Game/Code/Bags_And_Locking/Locking/BP_BagSlot.In Use` _array_element))
          (set `/Game/Code/Bags_And_Locking/Locking/BP_BagSlot.Hit` true _array_element)
          (set `/Game/Code/Bags_And_Locking/Locking/BP_BagSlot.In Use` true _array_element)
          (`SceneComponent.K2_SetWorldTransform` (`self.staticMesh`) (`self.GetTransform` _array_element) false false)
          (`PrimitiveComponent.SetSimulatePhysics` (`self.staticMesh`) false)
          (set `self.SlotHit` _array_element)
          (break))))
    (switch `/Game/Core/E_BagSizes` (`self.enum`)
      (:`NewEnumerator0`
        (`SceneComponent.SetVisibility` (`self.TextRender1`) true false)
        (`SceneComponent.SetVisibility` (`self.TextRender`) true false))
      (:`NewEnumerator2`
        (`SceneComponent.SetVisibility` (`self.TextRender3`) true false)
        (`SceneComponent.SetVisibility` (`self.TextRender2`) true false))
      (:`NewEnumerator3`
        (`SceneComponent.SetVisibility` (`self.TextRender5`) true false :!label _label)
        (`SceneComponent.SetVisibility` (`self.TextRender4`) true false))
      (:`NewEnumerator4`
        (goto _label)))
    (`TextRenderComponent.K2_SetText` (`self.TextRender`) (`|GetArrayItem` (`self.Text array`) (`KismetMathLibrary.Conv_ByteToInt` (`self.enum`))))
    (`TextRenderComponent.K2_SetText` (`self.TextRender1`) (`|GetArrayItem` (`self.Text array`) (`KismetMathLibrary.Conv_ByteToInt` (`self.enum`))))
    (`TextRenderComponent.K2_SetText` (`self.TextRender2`) (`|GetArrayItem` (`self.Text array`) (`KismetMathLibrary.Conv_ByteToInt` (`self.enum`))))
    (`TextRenderComponent.K2_SetText` (`self.TextRender3`) (`|GetArrayItem` (`self.Text array`) (`KismetMathLibrary.Conv_ByteToInt` (`self.enum`))))
    (`TextRenderComponent.K2_SetText` (`self.TextRender4`) (`|GetArrayItem` (`self.Text array`) (`KismetMathLibrary.Conv_ByteToInt` (`self.enum`))))
    (`TextRenderComponent.K2_SetText` (`self.TextRender5`) (`|GetArrayItem` (`self.Text array`) (`KismetMathLibrary.Conv_ByteToInt` (`self.enum`))))))

(event `self.GrabComponent.OnDropped`
  (bind _aspc_base (cast `/Game/Core/PC_Base` (`GameplayStatics.GetPlayerController` 0) :!pure true))
  (bind _aspc_base_2 (cast `/Game/Core/PC_Base` (`GameplayStatics.GetPlayerController` 0) :!pure true))
  (bind _asbp_bag_slot (cast `/Game/Code/Bags_And_Locking/Locking/BP_BagSlot` (`self.SlotHit`) :!pure true))
  (if (`/Game/Core/PC_Base.LoadingLevel?` (cast `/Game/Core/PC_Base` (`GameplayStatics.GetPlayerController` 0) :!pure true))
    (`PrimitiveComponent.SetEnableGravity` (`self.staticMesh`) true)
    (else
      (`PrimitiveComponent.SetEnableGravity` (`self.staticMesh`) false)))
  (if (`self.Overlap?`)
    (`/Game/Code/Bags_And_Locking/Locking/BP_BagSlot.Hide Hilight` (cast `/Game/Code/Bags_And_Locking/Locking/BP_BagSlot` (`self.SlotHit`) :!pure true))
    (`PrimitiveComponent.SetSimulatePhysics` (`self.staticMesh`) false)
    (`PrimitiveComponent.SetCollisionEnabled` (`self.staticMesh`) "NoCollision")
    (bind (_direction _fy_value) (`Timeline|rotator` :`NewTime` 1.0 :!via `PlayFromStart`)
      (:`Update`
        (`SceneComponent.K2_SetWorldRotation` (`self.staticMesh`) (`KismetMathLibrary.RLerp` (`SceneComponent.K2_GetComponentRotation` (`self.staticMesh`)) (`self.K2_GetActorRotation` _asbp_bag_slot) _fy_value) false false)
        (`/Game/Code/Bags_And_Locking/Locking/BP_BagSlot.Hide Hilight` _asbp_bag_slot :!label _label_2))
      (:`Finished`
        (bind (_direction_2 _fy_value_2) (`Timeline|Timeline` :`NewTime` 1.0 :!via `PlayFromStart`)
          (:`Update`
            (`SceneComponent.K2_SetWorldTransform` (`self.staticMesh`) (`KismetMathLibrary.TLerp` (`SceneComponent.K2_GetComponentToWorld` (`self.staticMesh`)) (`self.GetTransform` (cast `/Game/Code/Bags_And_Locking/Locking/BP_BagSlot` (`self.SlotHit`) :!pure true)) _fy_value_2) false false)
            (goto _label_2))
          (:`Finished`
            (bind _asbp_bag_slot_2 (cast `/Game/Code/Bags_And_Locking/Locking/BP_BagSlot` (`self.SlotHit`)))
            (set `/Game/Code/Bags_And_Locking/Locking/BP_BagSlot.Hit` true _asbp_bag_slot_2)
            (set `/Game/Code/Bags_And_Locking/Locking/BP_BagSlot.In Use` true _asbp_bag_slot_2)
            (`PrimitiveComponent.SetCollisionEnabled` (`self.staticMesh`) "QueryAndPhysics")
            (if (`/Game/Core/PC_Base.Trash task` (cast `/Game/Core/PC_Base` (`GameplayStatics.GetPlayerController` 0) :!pure true))
              (bind _outactors (`GameplayStatics.GetAllActorsOfClass` "/Game/Code/wristGadget/RenderTargets/BP_text.BP_text_C"))
              (for _array_element _outactors
                (bind _output_get (set `/Game/Core/PC_Base.IntDone` (+ (`/Game/Core/PC_Base.IntDone` _aspc_base_2) 1) _aspc_base_2))
                (`|VariableSetRef` (`.num1_15_5AD7C164784342C67D5998959EE4D18F` (break `/Game/Core/S_Print` (`|GetArrayItem` (`/Game/Code/wristGadget/RenderTargets/BP_text.Text` _array_element) 11))) (`KismetTextLibrary.Conv_IntToText` _output_get))
                (`/Game/Code/wristGadget/RenderTargets/BP_text.Update` _array_element)
                (if (== _output_get 3)
                  (set `/Game/Core/PC_Base.Trash task` false (cast `/Game/Core/PC_Base` (`GameplayStatics.GetPlayerController` 0) :!pure true))
                  (else
                    (break))))
              (else
                (bind _outactors_2 (`GameplayStatics.GetAllActorsOfClass` "/Game/Code/wristGadget/RenderTargets/BP_text.BP_text_C"))
                (for _array_element_2 _outactors_2
                  (bind _output_get_2 (set `/Game/Core/PC_Base.IntDone` (+ (`/Game/Core/PC_Base.IntDone` _aspc_base) 1) _aspc_base))
                  (`|VariableSetRef` (`.num1_15_5AD7C164784342C67D5998959EE4D18F` (break `/Game/Core/S_Print` (`|GetArrayItem` (`/Game/Code/wristGadget/RenderTargets/BP_text.Text` _array_element_2) 10))) (`KismetTextLibrary.Conv_IntToText` _output_get_2))
                  (`/Game/Code/wristGadget/RenderTargets/BP_text.Update` _array_element_2)
                  (break))))))))
    (else
      (`PrimitiveComponent.SetSimulatePhysics` (`self.staticMesh`) true))))

(event `self.GrabComponent.OnGrabbed`
  (bind _slothit (`self.SlotHit`))
  (bind _aspc_base (cast `/Game/Core/PC_Base` (`GameplayStatics.GetPlayerController` 0) :!pure true))
  (`/Engine/EditorBlueprintResources/StandardMacros.IsValid` _slothit
    (:`Is Valid`
      (bind _asbp_bag_slot (cast `/Game/Code/Bags_And_Locking/Locking/BP_BagSlot` _slothit))
      (if (`/Game/Code/Bags_And_Locking/Locking/BP_BagSlot.In Use` _asbp_bag_slot)
        (set `/Game/Code/Bags_And_Locking/Locking/BP_BagSlot.In Use` false _asbp_bag_slot)
        (set `/Game/Code/Bags_And_Locking/Locking/BP_BagSlot.Hit` false _asbp_bag_slot)
        (bind _outactors (`GameplayStatics.GetAllActorsOfClass` "/Game/Code/wristGadget/RenderTargets/BP_text.BP_text_C"))
        (for _array_element _outactors
          (bind _output_get (set `/Game/Core/PC_Base.IntDone` (+ (`/Game/Core/PC_Base.IntDone` _aspc_base) -1) _aspc_base))
          (`|VariableSetRef` (`.num1_15_5AD7C164784342C67D5998959EE4D18F` (break `/Game/Core/S_Print` (`|GetArrayItem` (`/Game/Code/wristGadget/RenderTargets/BP_text.Text` _array_element) 10))) (`KismetTextLibrary.Conv_IntToText` _output_get))
          (`/Game/Code/wristGadget/RenderTargets/BP_text.Update` _array_element))))))

(event `self.staticMesh.OnComponentBeginOverlap`
  (params (OverlappedComponent :type "PrimitiveComponent Object Reference") (OtherActor :type "Actor Object Reference") (OtherComp :type "PrimitiveComponent Object Reference") (OtherBodyIndex :type Integer) (bFromSweep :type Boolean) (SweepResult :type "HitResult Structure (by ref)"))
  (bind _asbp_bag_slot (cast `/Game/Code/Bags_And_Locking/Locking/BP_BagSlot` OtherActor))
  (if (`|EnumEquality` (`/Game/Code/Bags_And_Locking/Locking/BP_BagSlot.BagSizeEnum` _asbp_bag_slot) (`self.enum`))
    (if (not (`/Game/Code/Bags_And_Locking/Locking/BP_BagSlot.In Use` _asbp_bag_slot))
      (if (`self.Overlap?`)
        (bind _asbp_bag_slot_2 (cast `/Game/Code/Bags_And_Locking/Locking/BP_BagSlot` (`self.SlotHit`)))
        (set `/Game/Code/Bags_And_Locking/Locking/BP_BagSlot.Hit` false _asbp_bag_slot_2)
        (`/Game/Code/Bags_And_Locking/Locking/BP_BagSlot.Hide Hilight` _asbp_bag_slot_2))
      (bind _output_get (set `self.SlotHit` _asbp_bag_slot))
      (bind _asbp_bag_slot_3 (cast `/Game/Code/Bags_And_Locking/Locking/BP_BagSlot` _output_get))
      (`/Game/Code/Bags_And_Locking/Locking/BP_BagSlot.Add hilight` _asbp_bag_slot_3)
      (set `/Game/Code/Bags_And_Locking/Locking/BP_BagSlot.Hit` true _asbp_bag_slot_3)
      (set `self.Overlap?` true))))

(event `self.staticMesh.OnComponentEndOverlap`
  (params (OverlappedComponent :type "PrimitiveComponent Object Reference") (OtherActor :type "Actor Object Reference") (OtherComp :type "PrimitiveComponent Object Reference") (OtherBodyIndex :type Integer))
  (if (== OtherActor (`self.SlotHit`))
    (bind _asbp_bag_slot (cast `/Game/Code/Bags_And_Locking/Locking/BP_BagSlot` OtherActor))
    (if (`|EnumEquality` (`/Game/Code/Bags_And_Locking/Locking/BP_BagSlot.BagSizeEnum` _asbp_bag_slot) (`self.enum`))
      (bind _asbp_bag_slot_2 (cast `/Game/Code/Bags_And_Locking/Locking/BP_BagSlot` (`self.SlotHit`)))
      (set `/Game/Code/Bags_And_Locking/Locking/BP_BagSlot.Hit` false _asbp_bag_slot_2)
      (`/Game/Code/Bags_And_Locking/Locking/BP_BagSlot.Hide Hilight` _asbp_bag_slot_2)
      (set `self.Overlap?` false))))

(fn `UserConstructionScript`
  (switch `/Game/Core/E_BagSizes` (`self.enum`)
    (:`NewEnumerator0`
      (`StaticMeshComponent.SetStaticMesh` (`self.staticMesh`) "/Game/ArtAndMeshes/QasisModuleBags/Meshes/SM_Bags_SM_BagSmall.SM_Bags_SM_BagSmall"))
    (:`NewEnumerator2`
      (`StaticMeshComponent.SetStaticMesh` (`self.staticMesh`) "/Game/ArtAndMeshes/QasisModuleBags/Meshes/SM_Bags_SM_BagMedium.SM_Bags_SM_BagMedium"))
    (:`NewEnumerator3`
      (`StaticMeshComponent.SetStaticMesh` (`self.staticMesh`) "/Game/ArtAndMeshes/QasisModuleBags/Meshes/SM_Bags_SM_BagLarge.SM_Bags_SM_BagLarge"))
    (:`NewEnumerator4`
      (`StaticMeshComponent.SetStaticMesh` (`self.staticMesh`) "/Game/ArtAndMeshes/QasisModuleBags/Meshes/SM_Bags_SM_BagLargest.SM_Bags_SM_BagLargest"))))